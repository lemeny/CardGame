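; BP_Plane is a table actor that switches the player to a top-down view on approach, with an unfinished mechanic for tilting by block weight.
; Its PlayerDetection overlap blends to TopCamera and shows the cursor for BP_TPblock, then blends back on exit without hiding the cursor.
; Tick gathers every BP_Blocks but does nothing with them; CalculateCenter and block placement are stubs.
; UpdateMap would rotate the plane toward CenterPosition with debug output, but its EventGraph call never runs.
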(event `self.ReceiveBeginPlay`
  (set `self.TotalMass` 0.0)
  (set `self.WeightSum` (0.0 0.0 0.0)))

(event `self.ReceiveTick`
  (params (DeltaSeconds :type "Float (single-precision)"))
  (bind _outactors (`GameplayStatics.GetAllActorsOfClass` "/Game/BP/BP_Blocks.BP_Blocks_C"))
  (for _array_element _outactors
    _))

(event `self.PlayerDetection.OnComponentBeginOverlap`
  (params (OverlappedComponent :type "PrimitiveComponent Object Reference") (OtherActor :type "Actor Object Reference") (OtherComp :type "PrimitiveComponent Object Reference") (OtherBodyIndex :type Integer) (bFromSweep :type Boolean) (SweepResult :type "HitResult Structure (by ref)"))
  (bind _returnvalue (`GameplayStatics.GetPlayerController` 0))
  (`KismetSystemLibrary.PrintText` "near table" true true (struct :`A` 1.0))
  (cast `/Game/BP/PlayerCharacter/BP_TPblock` OtherActor)
  (`PlayerController.SetViewTargetWithBlend` _returnvalue (`ActorComponent.GetOwner` (`self.TopCamera`)) 2.0 "VTBlend_Linear" 0.0 false)
  (set `PlayerController.bShowMouseCursor` true _returnvalue))

(event `self.PlayerDetection.OnComponentEndOverlap`
  (params (OverlappedComponent :type "PrimitiveComponent Object Reference") (OtherActor :type "Actor Object Reference") (OtherComp :type "PrimitiveComponent Object Reference") (OtherBodyIndex :type Integer))
  (if (== OtherActor (`GameplayStatics.GetPlayerCharacter` 0))
    (`KismetSystemLibrary.PrintText` "Leave table")
    (bind _asbp_tpblock (cast `/Game/BP/PlayerCharacter/BP_TPblock` OtherActor))
    (`PlayerController.SetViewTargetWithBlend` (`GameplayStatics.GetPlayerController` 0) _asbp_tpblock 2.0 "VTBlend_Linear" 0.0 false)))

(fn `CalculateCenter`
  (`GameplayStatics.GetAllActorsOfClass` null))

(fn `PlaceBlockMode`
  (params (playercharacter :type "PlayerController Object Reference")))

(fn `RecieveBlock`)

(fn `UpdateMap`
  (bind _centerposition (`self.CenterPosition`))
  (`self.K2_SetActorRotation` (`KismetMathLibrary.Conv_VectorToRotator` _centerposition))
  (`KismetSystemLibrary.DrawDebugArrow` (`SceneComponent.GetUpVector` (`self.Cube`)) _centerposition 5.0 (struct :`G` 0.161411 :`B` 1.0 :`A` 1.0) 50.0 30.0)
  (`KismetSystemLibrary.PrintString` (`KismetStringLibrary.Conv_VectorToString` _centerposition))
  (`KismetSystemLibrary.PrintText` "Updated" true true (struct :`A` 1.0)))

(fn `UserConstructionScript`)