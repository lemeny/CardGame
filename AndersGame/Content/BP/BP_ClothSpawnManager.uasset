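; BP_ClothSpawnManager periodically spawns random cloth items at spawn locations in the level and registers each with the game mode's chaos system.
; On BeginPlay it fills a cloth pool from DT_ClothData, gathers BP_SpawnLocation actors and starts a looping timer.
; While ControlSpawn leaves spawning active, each tick of the timer spawns BP_Cloth with random row data near a random location, then passes that data to BP_TPGM_Chaos.AddChaos.
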(event `self.ReceiveBeginPlay`
  (`self.InitializeClothPool`)
  (`KismetSystemLibrary.K2_SetTimer` null "SpawnClothRandom" (`self.SpawnInterval`) true))

(fn `ControlSpawn`
  (params (OpenOrClose :type Boolean))
  (set `self.SpawnActivation` OpenOrClose))

(fn `InitializeClothPool`
  (bind _outrownames (`DataTableFunctionLibrary.GetDataTableRowNames` "/Game/Data/DT_ClothData.DT_ClothData"))
  (for _array_element _outrownames
    (bind _returnvalue (`|GetDataTableRow` "/Game/Data/DT_ClothData.DT_ClothData" _array_element)
      (:`then`
        (`KismetArrayLibrary.Array_Add` (`self.ClothPool`) _returnvalue)
        (bind _outactors (`GameplayStatics.GetAllActorsOfClass` "/Game/BP/BP_SpawnLocation.BP_SpawnLocation_C"))
        (set `self.SpawnLocation` _outactors)))))

(fn `SpawnClothRandom`
  (bind _spawnlocation (`self.SpawnLocation`))
  (bind _output (`|GetArrayItem` (`self.SpawnLocation`) (`KismetMathLibrary.RandomInteger` (`KismetArrayLibrary.Array_Length` _spawnlocation))))
  (bind _returnvalue_location (`KismetMathLibrary.BreakTransform` (`self.GetTransform` _output)))
  (if (`self.SpawnActivation`)
    (bind _output_get (set `self.SelectedCloth` (`KismetArrayLibrary.Array_Random` (`self.ClothPool`))))
    (`KismetArrayLibrary.Array_Add` (`self.SpawnedCloth`) _output_get)
    (if (`KismetArrayLibrary.Array_IsNotEmpty` _spawnlocation)
      (`/Engine/EditorBlueprintResources/StandardMacros.IsValid` _output
        (:`Is Valid`
          (`AddComponent|NODE_AddRandomVector-0`)
          (`|SpawnActorFromClass` "/Game/BP/BP_Cloth.BP_Cloth_C" (`KismetMathLibrary.Conv_VectorToTransform` (+ _returnvalue_location (* (`KismetMathLibrary.RandomUnitVector`) 5.0))) "Undefined" "MultiplyWithRoot" null _output_get null)
          (bind _asbp_tpgm_chaos (cast `/Game/BP/BP_TPGM_Chaos` (`GameplayStatics.GetGameMode`)))
          (`/Game/BP/BP_TPGM_Chaos.AddChaos` _asbp_tpgm_chaos _output_get))))))

(fn `UserConstructionScript`)