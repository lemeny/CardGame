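; Inventory manager Blueprint that sets up the occupancy grid for a backpack-based inventory.
; On BeginPlay, Initialization builds OccupiedGrid from the GridX and GridY dimensions of BakcPackType, with every cell marked unoccupied.
; The 2D grid is an array of SOccupiedGrid structs, each wrapping a boolean array.
; Only this setup is implemented; a debug print of the cells is left unconnected.
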(event `self.ReceiveBeginPlay`
  (`self.Initialization`))

(fn `Initialization`
  (bind (_bakcpacktype_backpackid _bakcpacktype_displayname _bakcpacktype_gridx _bakcpacktype_gridy) (break `/Game/InventorySystem/S_BackPack` (`self.BakcPackType`)))
  (set `self.OccupiedGrid` (`self.OccupiedGrid`))
  (for _ (range _bakcpacktype_gridx)
    (`KismetArrayLibrary.Array_Clear` (`self.RowArray`))
    (for _ (range _bakcpacktype_gridy)
      (`KismetArrayLibrary.Array_Add` (`self.RowArray`)))
    (`KismetArrayLibrary.Array_Add` (`self.OccupiedGrid`) (make `/Game/InventorySystem/S_OccupiedGrid` (`self.RowArray`)))))

(fn `UserConstructionScript`)